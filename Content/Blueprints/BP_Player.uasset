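; Player Blueprint that rotates its root in yaw, either in an idle motion or in 90-degree turns, with a 2D ambient sound.
; The IdleRot timeline loops while Idle is set, then EndRotate steps yaw back to zero through a self-calling Delay loop.
; Rotate90Deg uses a timeline to add a direction-scaled offset to the starting yaw.
; SetAmbientVolume switches to the loud level during turns and the return to zero, then restores it.
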(event `self.ReceiveBeginPlay`
  (`self.Rotate`)
  (cast `/Game/Blueprints/BP_GameInstance` (`GameplayStatics.GetGameInstance`))
  (bind _returnvalue (`GameplayStatics.CreateSound2D` "/Game/Audio/SFX/ambient.ambient" 1.0 1.0 0.0 null))
  (bind _output_get (set `self.AmbientSound` _returnvalue))
  (set `self.AmbientVolumeOriginal` (`AudioComponent.VolumeMultiplier` _output_get))
  (`AudioComponent.Play` _output_get 0.0))

(event `Rotate`
  (bind _idle (`self.Idle`))
  (bind (_direction _idleval) (`Timeline|IdleRot` :!via `PlayFromStart` :!label _label)
    (:`Update`
      (if _idle
        (`SceneComponent.K2_SetRelativeRotation` (`self.DefaultSceneRoot`) (`KismetMathLibrary.MakeRotator` 0.0 0.0 _idleval) false false)
        (else
          (`self.EndRotate` :!label _label_2)
          (goto _label :!via `Stop`))))
    (:`Finished`
      (if _idle
        (`KismetSystemLibrary.Delay` 0.001)
        (`self.Rotate`)
        (else
          (goto _label_2))))))

(event `EndRotate`
  (bind _defaultsceneroot (`self.DefaultSceneRoot`))
  (bind (_relativerotation_roll _relativerotation_pitch _relativerotation_yaw) (`KismetMathLibrary.BreakRotator` (`SceneComponent.RelativeRotation` _defaultsceneroot)))
  (bind _returnvalue (`KismetMathLibrary.Conv_FloatToDouble` _relativerotation_yaw))
  (bind _returnvalue_2 (`KismetMathLibrary.Conv_FloatToDouble` _relativerotation_yaw))
  (bind _returnvalue_3 (* (`self.IdleEndSpeed`) (`KismetMathLibrary.Conv_FloatToDouble` (`GameplayStatics.GetWorldDeltaSeconds`))))
  (`self.SetAmbientVolume` true)
  (if (> _returnvalue -0.1)
    (if (< _returnvalue 0.1)
      (`self.SetAmbientVolume` false)
      (else
        (`SceneComponent.K2_SetRelativeRotation` _defaultsceneroot (`KismetMathLibrary.MakeRotator` _relativerotation_roll _relativerotation_pitch (`KismetMathLibrary.FClamp` (- _returnvalue_2 _returnvalue_3) 0.0 180.0)) false false)
        (`KismetSystemLibrary.Delay` 0.001 :!label _label_3)
        (`self.EndRotate`)))
    (else
      (`SceneComponent.K2_SetRelativeRotation` _defaultsceneroot (`KismetMathLibrary.MakeRotator` _relativerotation_roll _relativerotation_pitch (`KismetMathLibrary.FClamp` (+ _returnvalue_2 _returnvalue_3) -180.0 0.0)) false false)
      (goto _label_3))))

(event `Rotate90Deg`
  (params (dir :type "Float (double-precision)"))
  (bind _defaultsceneroot (`self.DefaultSceneRoot`))
  (`self.SetAmbientVolume` true)
  (bind _output_get (set `self.TempRot` (`SceneComponent.RelativeRotation` _defaultsceneroot)))
  (bind (_direction _time) (`Timeline|90Deg` :!via `PlayFromStart`)
    (:`Update`
      (`SceneComponent.K2_SetRelativeRotation` _defaultsceneroot (`KismetMathLibrary.MakeRotator` (.roll _output_get) (.pitch _output_get) (+ (* (`KismetMathLibrary.Conv_FloatToDouble` _time) dir) (.yaw _output_get))) false false))
    (:`Finished`
      (`self.SetAmbientVolume` false))))

(fn `SetAmbientVolume`
  (params (IsLoud :type Boolean))
  (bind _ambientsound (`self.AmbientSound`))
  (if IsLoud
    (`AudioComponent.SetVolumeMultiplier` _ambientsound (`self.AmbientVolumeMultiplier`))
    (else
      (`AudioComponent.SetVolumeMultiplier` _ambientsound (`self.AmbientVolumeOriginal`)))))

(fn `UserConstructionScript`
  (`SceneComponent.K2_SetWorldTransform` (`self.DefaultSceneRoot`) (`KismetMathLibrary.MakeTransform` (0.0 0.0 0.0)) false false))