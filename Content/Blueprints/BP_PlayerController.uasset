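; Player controller for a touch-driven block-building game that places and breaks blocks and handles inactivity.
; The first touch wakes the game; later touches line-trace, breaking non-bedrock blocks at selection index zero, otherwise spawning the selected block along the hit normal.
; Logs align to that normal, and signs reject placement.
; Touches refresh two timers: one starts idle rotation and hides the block bar, the other takes a screenshot and restarts the game.
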(event `InputTouch`
  (params (Location :type "Vector Structure") (FingerIndex :type "ETouchIndex Enum"))
  (bind _selectedblockindex (`self.SelectedBlockIndex`))
  (bind (_worldposition _worlddirection) (`GameplayStatics.DeprojectScreenToWorld` self (`KismetMathLibrary.Conv_VectorToVector2D` Location)))
  (:`Pressed`
    (switch `int` (`self.SwitchInt`)
      (:`0`
        (`self.InitialClick`)
        (`self.RefreshTimer`))
      (:`1`
        (bind (_outhit _returnvalue) (`KismetSystemLibrary.LineTraceSingle` _worldposition (+ _worldposition (* _worlddirection 100000.0)) "TraceTypeQuery1"))
        (if _returnvalue
          (if (`KismetMathLibrary.Conv_IntToBool` _selectedblockindex)
            (cast `/Game/Blueprints/Blocks/BP_Sign` (`.HitActor` (`GameplayStatics.BreakHitResult` _outhit))
              (:`CastFailed`
                (bind _returnvalue_2 (`|SpawnActorFromClass` (`|GetArrayItem` (`self.AvailableBlocks`) _selectedblockindex) (`KismetMathLibrary.MakeTransform` (+ (* (`.Normal` (`GameplayStatics.BreakHitResult` _outhit)) (200.0 200.0 200.0)) (`self.K2_GetActorLocation` (`.HitActor` (`GameplayStatics.BreakHitResult` _outhit))))) "Undefined" "OverrideRootScale" null null))
                (`/Game/Blueprints/BP_Block.PlayPlaceSound` _returnvalue_2)
                (bind _asbp_log (cast `/Game/Blueprints/Blocks/BP_Log` _returnvalue_2)
                  (:`then`
                    (`self.K2_SetActorRotation` _asbp_log (`KismetMathLibrary.MakeRotator` (* (.y (`.Normal` (`GameplayStatics.BreakHitResult` _outhit))) 90.0) (* (.x (`.Normal` (`GameplayStatics.BreakHitResult` _outhit))) 90.0)) false))
                  (:`CastFailed`
                    _))))
            (else
              (bind _asbp_block (cast `/Game/Blueprints/BP_Block` (`.HitActor` (`GameplayStatics.BreakHitResult` _outhit))))
              (cast `/Game/Blueprints/Blocks/BP_Bedrock` _asbp_block
                (:`then`
                  _)
                (:`CastFailed`
                  (`/Game/Blueprints/BP_Block.PlayBreakSound` _asbp_block)
                  (`self.K2_DestroyActor` _asbp_block))))))
        (`KismetSystemLibrary.Delay` 1.0)
        (`self.RefreshTimer`)))))

(event `InitialClick`
  (bind _asbp_game_mode (cast `/Game/Blueprints/BP_GameMode` (`GameplayStatics.GetGameMode`)))
  (`/Game/Blueprints/BP_UI.ShowBlockBar` (`/Game/Blueprints/BP_GameMode.BP_UI` _asbp_game_mode))
  (set `self.SwitchInt` 1)
  (set `/Game/Blueprints/BP_Player.Idle` false (`self.BP_Player`)))

(event `StartIdle`
  (bind _bp_player (`self.BP_Player`))
  (bind _asbp_game_mode (cast `/Game/Blueprints/BP_GameMode` (`GameplayStatics.GetGameMode`)))
  (`/Game/Blueprints/BP_UI.HideBlockBar` (`/Game/Blueprints/BP_GameMode.BP_UI` _asbp_game_mode))
  (set `self.SwitchInt` 0)
  (set `/Game/Blueprints/BP_Player.Idle` true _bp_player)
  (`/Game/Blueprints/BP_Player.EndRotate` _bp_player)
  (`KismetSystemLibrary.Delay` 1.0)
  (`/Game/Blueprints/BP_Player.Rotate` _bp_player))

(event `RefreshTimer`
  (`KismetSystemLibrary.K2_ClearAndInvalidateTimerHandle` (`self.IdleTimer`))
  (`KismetSystemLibrary.K2_ClearAndInvalidateTimerHandle` (`self.RestartTimer`))
  (bind _returnvalue (`KismetSystemLibrary.K2_SetTimerDelegate` (delegate `StartIdle`) (`self.TimeTillIdle`)))
  (set `self.IdleTimer` _returnvalue)
  (bind _returnvalue_2 (`KismetSystemLibrary.K2_SetTimerDelegate` (delegate `Restart`) (`self.TimeTillRestart`)))
  (set `self.RestartTimer` _returnvalue_2))

(event `Restart`
  (bind _bp_player (`self.BP_Player`))
  (set `/Game/Blueprints/BP_Player.Idle` false _bp_player)
  (`/Game/Blueprints/BP_Player.EndRotate` _bp_player)
  (`KismetSystemLibrary.Delay` 1.0)
  (`self.TakeScreenshot`)
  (bind _asbp_game_mode (cast `/Game/Blueprints/BP_GameMode` (`GameplayStatics.GetGameMode`)))
  (`GameMode.RestartGame` _asbp_game_mode))

(event `self.ReceiveBeginPlay`
  (bind _asbp_player (cast `/Game/Blueprints/BP_Player` (`GameplayStatics.GetPlayerPawn` 0)))
  (set `self.BP_Player` _asbp_player))

(fn `TakeScreenshot`
  (`KismetSystemLibrary.ExecuteConsoleCommand` "HighResShot 540x960" null))

(fn `UserConstructionScript`)